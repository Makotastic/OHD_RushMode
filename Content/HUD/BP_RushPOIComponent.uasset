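; BP_RushPOIComponent is an actor component that registers its owner as a point of interest on the local player's minimap.
; Where cosmetic events can run, BeginPlay starts a looping timer that polls because controller and minimap references may be invalid, especially when joining.
; Once references, both team numbers and the player state are valid, it stops polling and adds the POI if not already registered.
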(event Custom|TryRegisterPOI
  ;[1 1 0] @NOTE: Keep attempting to setup and register our POI. References like the minimap and HUD can be invalid for various reasons especially when joining.
  (bind _ballvalid (POI|Helpers|GetRequiredRefs))
  (if _ballvalid
    ;[1 1 1] Ensure our local PC and our POI both have valid team numbers.
    (if (not (or (== (Class|DFBlueprintFunctions|GetTeamNum (Variables|POI|Refs|GetLocalPC)) (Utilities|Enum|LiteralenumEHDTeam "NoTeam")) (== (POI|GetPOITeamNum) (Utilities|Enum|LiteralenumEHDTeam "NoTeam"))))
      ;[1 1 1] Check if our player state is valid. Used to check for squad status, etc.
      (Utilities|IsValid (Default|GetHDPlayerState (Variables|POI|Refs|GetLocalPC))
        (:Is%20Valid
          (Utilities|Time|ClearandInvalidateTimerbyHandle (Variables|POI|Refs|GetTryRegisterPOI_Timer)) ; @NOTE: We have all our required references that we need. Stop polling.
          (Utilities|IsValid (Variables|POI|Refs|GetPOI) ; @NOTE: Register ourselves if we are not already.
            (:Is%20Not%20Valid
              (bind _returnvalue (Class|DFMinimap|AddNewPOI (Variables|POI|Refs|GetMinimap) (Components|GetOwner)))
              (Variables|POI|Refs|SetPOI _returnvalue))))))))

(event EventBeginPlay
  ;[1 1 0] @NOTE: Keep attempting to setup and register our POI. References like the minimap and HUD can be invalid for various reasons especially when joining.
  (Networking|CanExecuteCosmeticEvents
    (:True
      (bind _returnvalue (Utilities|Time|SetTimerbyEvent (delegate Custom|TryRegisterPOI) (Variables|POI|Settings|GetTryRegisterPOI_IntervalSeconds) true))
      (Variables|POI|Refs|SetTryRegisterPOI_Timer _returnvalue))))

(fn GetRequiredRefs
  (bind _hdpc (CallFunction|GetHDPlayerControllerBP))
  (Variables|POI|Refs|GetLocalPC
    (:then
      (Variables|POI|Refs|GetMinimap
        (:then
          (return true))
        (:else
          _)))
    (:else
      (Utilities|IsValid _hdpc
        (:Is%20Valid
          (Variables|POI|Refs|SetLocalPC _hdpc))
        (:Is%20Not%20Valid
          (return false)))))
  (Utilities|IsValid (Default|GetMinimapWidget (Variables|POI|Refs|GetLocalPC))
    (:Is%20Valid
      (Variables|POI|Refs|SetMinimap (Default|GetMinimapWidget (Variables|POI|Refs|GetLocalPC)))
      (return true))
    (:Is%20Not%20Valid
      (return false))))

(fn GetPOITeamNum
  (return (Class|DFBlueprintFunctions|GetTeamNum (Components|GetOwner))))