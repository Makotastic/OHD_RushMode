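; HUD for Rush mode that shows screen-space markers over the current tier's uncaptured rush points.
; It waits for RushGameState setup, spawns marker widgets into the root HUD container, and rebuilds them on tier changes or HUD reset.
; Player team changes switch markers between attacker and defender appearance.
; Tick projects markers to screen, fading them near screen center with a sigmoid curve and pulsing armed points with a sine wave.
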(event Custom|Begin
  (bind _asrush_game_state (Utilities|Casting|CastToRushGameState (Game|GetGameState) :!label _label)
    (:then
      (bind _output_get (Variables|Default|SetGamestate _asrush_game_state))
      (if (Variables|/RushMode/Core/RushGameState.RushGameState_C|GetDoneSetup _output_get)
        (Variables|Default|SetAttackingTeam (Variables|/RushMode/Core/RushGameState.RushGameState_C|GetAttackingTeam _output_get))
        (CallFunction|AddRushMarkers)
        (bind _asbp_hdplayer_controller_base (Utilities|Casting|CastToBP_HDPlayerControllerBase (Game|GetPlayerController 0)))
        (CallFunction|UpdateMarkerImages (Class|DFBlueprintFunctions|GetTeamNum _asbp_hdplayer_controller_base))
        (EventDispatchers|BindEventtoOnPlayerTeamNumUpdated _asbp_hdplayer_controller_base (EventDispatchers|CreateEvent :!event BPRushHUDAutoGenFunc))
        (EventDispatchers|BindEventtoTierUpdated (Variables|Default|GetGamestate) (EventDispatchers|CreateEvent :!event TeirUpdated))
        (EventDispatchers|UnbindEventfromSetupDone (Variables|Default|GetGamestate) (EventDispatchers|CreateEvent :!event Custom|SetupCallBack))
        (else
          (EventDispatchers|BindEventtoSetupDone _output_get (delegate Custom|SetupCallBack)))))
    (:CastFailed
      (Utilities|FlowControl|RetriggerableDelay 0.2)
      (goto _label))))

(event Custom|SetupCallBack
  (Variables|Default|SetAttackingTeam (Variables|/RushMode/Core/RushGameState.RushGameState_C|GetAttackingTeam (stale Custom|Begin _output_get)))
  (CallFunction|AddRushMarkers)
  (bind _asbp_hdplayer_controller_base (Utilities|Casting|CastToBP_HDPlayerControllerBase (Game|GetPlayerController 0)))
  (CallFunction|UpdateMarkerImages (Class|DFBlueprintFunctions|GetTeamNum _asbp_hdplayer_controller_base))
  (EventDispatchers|BindEventtoOnPlayerTeamNumUpdated _asbp_hdplayer_controller_base (EventDispatchers|CreateEvent :!event BPRushHUDAutoGenFunc))
  (EventDispatchers|BindEventtoTierUpdated (Variables|Default|GetGamestate) (EventDispatchers|CreateEvent :!event TeirUpdated))
  (EventDispatchers|UnbindEventfromSetupDone (Variables|Default|GetGamestate) (EventDispatchers|CreateEvent :!event Custom|SetupCallBack)))

(event Custom|ResetHUD
  (CallFunction|HideHUDWidget true)
  (CallFunction|ShowHUDWidget)
  (CallFunction|RemoveAllMarkers)
  (CallFunction|Begin))

(event EventBeginPlay
  (|CallParentFunction)
  (CallFunction|Begin))

(event Collision|EventActorBeginOverlap
  (params (OtherActor :type Actor%20Object%20Reference))
  (|CallParentFunction OtherActor) ; This node is disabled and will not be called.\nDrag off pins to build functionality.
)

(event EventTick
  (params (DeltaSeconds :type Float%20%28single-precision%29))
  (|CallParentFunction DeltaSeconds)
  (Variables|Default|SetClock (+ DeltaSeconds (Variables|Default|GetClock)))
  (CallFunction|TickRushMarkers))

(event EventEndPlay
  (params (EndPlayReason :type EEndPlayReason%20Enum :default "Destroyed"))
  (bind _asbp_hdplayer_controller_base (Utilities|Casting|CastToBP_HDPlayerControllerBase (Game|GetPlayerController 0)))
  (EventDispatchers|UnbindEventfromOnPlayerTeamNumUpdated _asbp_hdplayer_controller_base (EventDispatchers|CreateEvent :!event BPRushHUDAutoGenFunc))
  (EventDispatchers|UnbindEventfromTierUpdated (Variables|Default|GetGamestate) (EventDispatchers|CreateEvent :!event TeirUpdated)))

(fn ConstructionScript
  (|CallParentFunction))

(fn AddRushMarkers
  (for (_array_element _array_index) (Utilities|Struct|BreakRushTier (Utilities|Array|Get(acopy) (Variables|/RushMode/Core/RushGameState.RushGameState_C|GetRushTierArray (Variables|Default|GetGamestate)) (Math|Conversions|ToInteger(Byte) (Variables|/RushMode/Core/RushGameState.RushGameState_C|GetCurrentTier (Variables|Default|GetGamestate)))))
    (if (not (Variables|/RushMode/Core/RushPoint.RushPoint_C|GetCaptured _array_element))
      (bind _returnvalue (UserInterface|CreateWidget (Variables|Default|GetRushPointMarker) (Game|GetPlayerController 0) _array_element self (Math|Conversions|ToByte(Integer) _array_index)))
      (bind _aswbp_rush_root_hudcontainer (Utilities|Casting|CastToWBP_RushRootHUDContainer (CallFunction|GetValidRootHUDContainer)))
      (bind _returnvalue_2 (Widget|Panel|AddChild (Variables|/RushMode/HUD/WBP_RushRootHUDContainer.WBP_RushRootHUDContainer_C|GetHUDContainer _aswbp_rush_root_hudcontainer) _returnvalue))
      (bind _ascanvas_panel_slot (Utilities|Casting|CastToCanvasPanelSlot _returnvalue_2))
      (Utilities|Array|Add (Variables|Default|GetMarkers) (Utilities|Struct|MakeRushPointMarkerData (Math|Conversions|ToByte(Integer) _array_index) _returnvalue _ascanvas_panel_slot)))))

(fn TickRushMarkers
  (for _array_element (Variables|Default|GetMarkers)
    (if (.ReturnValue (Class|WidgetLayoutLibrary|ProjectWorldLocationtoWidgetPosition (Variables|Default|GetPlayerOwner) (Transformation|GetWorldLocation (Variables|/RushMode/Core/RushPoint.RushPoint_C|GetStaticMesh (Variables|/RushMode/HUD/RushPointMarker.RushPointMarker_C|GetRushPoint (.RushPointMarker (Utilities|Struct|BreakRushPointMarkerData _array_element))))) true))
      (Widget|SetVisibility (.RushPointMarker (Utilities|Struct|BreakRushPointMarkerData _array_element)) "Visible")
      (Class|CanvasPanelSlot|SetPosition (.CanvasPanelSlot (Utilities|Struct|BreakRushPointMarkerData _array_element)) (.ScreenPosition (Class|WidgetLayoutLibrary|ProjectWorldLocationtoWidgetPosition (Variables|Default|GetPlayerOwner) (Transformation|GetWorldLocation (Variables|/RushMode/Core/RushPoint.RushPoint_C|GetStaticMesh (Variables|/RushMode/HUD/RushPointMarker.RushPointMarker_C|GetRushPoint (.RushPointMarker (Utilities|Struct|BreakRushPointMarkerData _array_element))))) true)))
      (if (Variables|/RushMode/Core/RushPoint.RushPoint_C|GetArmed (Variables|/RushMode/HUD/RushPointMarker.RushPointMarker_C|GetRushPoint (.RushPointMarker (Utilities|Struct|BreakRushPointMarkerData _array_element))))
        (Widget|SetRenderOpacity (.RushPointMarker (Utilities|Struct|BreakRushPointMarkerData _array_element)) (* (/ (+ (Math|Trig|Sin(Radians) (* (Variables|Default|GetClock) 6.0)) 1.0) 2.0) (select (> (Math|Vector2D|Vector2DLength (/ (- (.ScreenPosition (Class|GameplayStatics|ProjectWorldtoScreen (Variables|Default|GetPlayerOwner) (Transformation|GetWorldLocation (Variables|/RushMode/Core/RushPoint.RushPoint_C|GetStaticMesh (Variables|/RushMode/HUD/RushPointMarker.RushPointMarker_C|GetRushPoint (.RushPointMarker (Utilities|Struct|BreakRushPointMarkerData _array_element))))) false)) (/ (Viewport|GetViewportSize) 2.0)) (Viewport|GetViewportSize))) 0.2) 1.0 (Math|Float|Clamp(Float) (+ (/ 1.0 (+ (Class|KismetMathLibrary|Exp (* (+ (Math|Vector2D|Vector2DLength (/ (- (.ScreenPosition (Class|GameplayStatics|ProjectWorldtoScreen (Variables|Default|GetPlayerOwner) (Transformation|GetWorldLocation (Variables|/RushMode/Core/RushPoint.RushPoint_C|GetStaticMesh (Variables|/RushMode/HUD/RushPointMarker.RushPointMarker_C|GetRushPoint (.RushPointMarker (Utilities|Struct|BreakRushPointMarkerData _array_element))))) false)) (/ (Viewport|GetViewportSize) 2.0)) (Viewport|GetViewportSize))) -0.05) -7e+01)) 1.0)) 0.0) 0.1 1.0))))
        (else
          (Widget|SetRenderOpacity (.RushPointMarker (Utilities|Struct|BreakRushPointMarkerData _array_element)) (select (> (Math|Vector2D|Vector2DLength (/ (- (.ScreenPosition (Class|GameplayStatics|ProjectWorldtoScreen (Variables|Default|GetPlayerOwner) (Transformation|GetWorldLocation (Variables|/RushMode/Core/RushPoint.RushPoint_C|GetStaticMesh (Variables|/RushMode/HUD/RushPointMarker.RushPointMarker_C|GetRushPoint (.RushPointMarker (Utilities|Struct|BreakRushPointMarkerData _array_element))))) false)) (/ (Viewport|GetViewportSize) 2.0)) (Viewport|GetViewportSize))) 0.2) 1.0 (Math|Float|Clamp(Float) (+ (/ 1.0 (+ (Class|KismetMathLibrary|Exp (* (+ (Math|Vector2D|Vector2DLength (/ (- (.ScreenPosition (Class|GameplayStatics|ProjectWorldtoScreen (Variables|Default|GetPlayerOwner) (Transformation|GetWorldLocation (Variables|/RushMode/Core/RushPoint.RushPoint_C|GetStaticMesh (Variables|/RushMode/HUD/RushPointMarker.RushPointMarker_C|GetRushPoint (.RushPointMarker (Utilities|Struct|BreakRushPointMarkerData _array_element))))) false)) (/ (Viewport|GetViewportSize) 2.0)) (Viewport|GetViewportSize))) -0.05) -7e+01)) 1.0)) 0.0) 0.1 1.0)))))
      (else
        (Widget|SetVisibility (.RushPointMarker (Utilities|Struct|BreakRushPointMarkerData _array_element)) "Hidden")))))

(fn RemoveMarker
  (params (Id :type Byte))
  (bind (_arrayindex _arrayelement) (Utilities|Array|ReverseforEachLoop (Variables|Default|GetMarkers))
    (:LoopBody
      (if (== Id (Utilities|Struct|BreakRushPointMarkerData _arrayelement))
        (Utilities|Array|RemoveIndex (Variables|Default|GetMarkers) _arrayindex)))))

(fn BPRushHUDAutoGenFunc
  (params (LastTeamNum :type Byte) (NewTeamNum :type Byte))
  (CallFunction|UpdateMarkerImages NewTeamNum))

(fn TeirUpdated
  (params (Tier :type Byte))
  (Variables|Default|SetTier Tier)
  (for _array_element (Variables|Default|GetMarkers)
    (Utilities|IsValid (Utilities|Struct|BreakRushPointMarkerData _array_element)
      (:Is%20Valid
        (Widget|RemovefromParent (Utilities|Struct|BreakRushPointMarkerData _array_element)))))
  (Utilities|Array|Clear (Variables|Default|GetMarkers))
  (CallFunction|AddRushMarkers)
  (CallFunction|UpdateMarkerImages (Class|DFBlueprintFunctions|GetTeamNum (Game|GetPlayerController 0))))

(fn UpdateMarkerImages
  (params (CurrentTeam :type Byte))
  (for _array_element (Variables|Default|GetMarkers)
    (Default|UpdateMarker (Utilities|Struct|BreakRushPointMarkerData _array_element) (== CurrentTeam (Variables|Default|GetAttackingTeam)))))

(fn RemoveAllMarkers
  (bind _arrayelement (Utilities|Array|ReverseforEachLoop (Variables|Default|GetMarkers))
    (:LoopBody
      (Widget|RemovefromParent (.RushPointMarker (Utilities|Struct|BreakRushPointMarkerData _arrayelement))))
    (:Completed
      (Utilities|Array|Clear (Variables|Default|GetMarkers)))))